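; BP_PawnController is a player pawn with an orthographic camera, held to the X = 0 plane every tick.
; Interact toggles use of the registered InteractRef through use/unuse messages, zooming out while interacting and back in on exit.
; The CameraZoom timeline blends spring arm height and ortho width.
; Five physics handles follow the HoldObject point each tick and can be released by index; grabbing happens outside this graph.
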(event `self.ReceiveBeginPlay`
  (set `self.ArrayHandlePhysics` (`|MakeArray` (`self.PhysicsHandle`) (`self.PhysicsHandle1`) (`self.PhysicsHandle2`) (`self.PhysicsHandle3`) (`self.PhysicsHandle4`)))
  (`self.SetCameraPosition` true))

(event `Interact`
  (if (`self.IsInteract`)
    (bind _interactref (`self.InteractRef`)
      (:`then`
        (message `/Game/Assets/Blueprints/Interface/BPI_Interact.UnUse` _interactref)
        (set `self.IsInteract` false)
        (`self.SetCameraPosition` true))
      (:`else`))
    (else
      (bind _interactref_2 (`self.InteractRef`)
        (:`then`
          (message `/Game/Assets/Blueprints/Interface/BPI_Interact.Use` _interactref_2 self)
          (set `self.IsInteract` true)
          (`self.SetCameraPosition` false))
        (:`else`)))))

(event `SetCameraPosition`
  (params (Bool :type Boolean))
  (if Bool
    (bind (_direction _float) (`Timeline|CameraZoom` :!via `PlayFromStart` :!label _label)
      (:`Update`
        (set `SpringArmComponent.SocketOffset` (`KismetMathLibrary.MakeVector` 0.0 0.0 (`KismetMathLibrary.Lerp` 450.0 150.0 _float)) (`self.SpringArm`))
        (`CameraComponent.SetOrthoWidth` (`self.Camera`) (`KismetMathLibrary.Lerp` 4000.0 2000.0 _float))))
    (else
      (goto _label :!via `ReverseFromEnd`))))

(event `/Game/Assets/Blueprints/Interface/BPI_Interact.SetInteract`
  (params (Actor :type "Actor Object Reference"))
  (set `self.InteractRef` Actor))

(event `self.ReceiveTick`
  (params (DeltaSeconds :type "Float (single-precision)"))
  (bind (_returnvalue_x _returnvalue_y _returnvalue_z) (`KismetMathLibrary.BreakVector` (`self.K2_GetActorLocation`)))
  (for _array_element (`self.ArrayHandlePhysics`)
    (`PhysicsHandleComponent.SetTargetLocation` _array_element (`SceneComponent.K2_GetComponentLocation` (`self.HoldObject`))))
  (`self.K2_SetActorLocation` (`KismetMathLibrary.MakeVector` 0.0 _returnvalue_y _returnvalue_z)))

(event `ReleaseByIndex`
  (params (Index :type Integer))
  (`PhysicsHandleComponent.ReleaseComponent` (`|GetArrayItem` (`self.ArrayHandlePhysics`) Index)))

(fn `UserConstructionScript`)