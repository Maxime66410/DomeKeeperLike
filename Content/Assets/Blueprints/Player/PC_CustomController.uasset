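; Player controller that turns Enhanced Input into movement, interaction and firing for the possessed BP_PawnController.
; It adds the default mapping context on BeginPlay and caches the pawn on possession.
; Move input drives floating movement in the YZ plane, or rotates the dome on the pawn's InteractRef while interacting.
; Interact calls the pawn, and Fire starts or cancels firing on InteractRef during interaction.
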(event `self.ReceiveBeginPlay`
  (bind _returnvalue (subsystem `EnhancedInputLocalPlayerSubsystem`))
  (`/Engine/EditorBlueprintResources/StandardMacros.IsValid` _returnvalue
    (:`Is Valid`
      (`EnhancedInputSubsystemInterface.AddMappingContext` _returnvalue "/Game/Assets/Blueprints/Input/IMC_Defaults.IMC_Defaults" 0 (struct)))))

(event `self.ReceivePossess`
  (params (PossessedPawn :type "Pawn Object Reference"))
  (bind _asbp_pawn_controller (cast `/Game/Assets/Blueprints/Player/BP_PawnController` PossessedPawn))
  (set `self.PawnRef` _asbp_pawn_controller))

(event `EnhancedInput|/Game/Assets/Blueprints/Input/IA_Move`
  (params (ActionValue :type "Vector2D Structure") (ElapsedSeconds :type "Float (double-precision)") (TriggeredSeconds :type "Float (double-precision)") (InputAction :type "InputAction Object Reference" :default "/Game/Assets/Blueprints/Input/IA_Move.IA_Move"))
  (:`Triggered`
    (bind _pawnref (`self.PawnRef`)
      (:`then`
        (if (not (`/Game/Assets/Blueprints/Player/BP_PawnController.IsInteract` _pawnref))
          (`PawnMovementComponent.AddInputVector` (`/Game/Assets/Blueprints/Player/BP_PawnController.FloatingPawnMovement` _pawnref) (`KismetMathLibrary.MakeVector` 0.0 ActionValue_X ActionValue_Y) false)
          (else
            (bind _interactref (`/Game/Assets/Blueprints/Player/BP_PawnController.InteractRef` _pawnref)
              (:`then`
                (message `/Game/Assets/Blueprints/Interface/BPI_Interact.RotateDome` _interactref ActionValue_X))
              (:`else`)))))
      (:`else`))))

(event `EnhancedInput|/Game/Assets/Blueprints/Input/IA_Interact`
  (params (ActionValue :type Boolean) (ElapsedSeconds :type "Float (double-precision)") (TriggeredSeconds :type "Float (double-precision)") (InputAction :type "InputAction Object Reference" :default "/Game/Assets/Blueprints/Input/IA_Interact.IA_Interact"))
  (:`Started`
    (bind _pawnref (`self.PawnRef`)
      (:`then`
        (`/Game/Assets/Blueprints/Player/BP_PawnController.Interact` _pawnref))
      (:`else`))))

(event `EnhancedInput|/Game/Assets/Blueprints/Input/IA_Fire`
  (params (ActionValue :type Boolean) (ElapsedSeconds :type "Float (double-precision)") (TriggeredSeconds :type "Float (double-precision)") (InputAction :type "InputAction Object Reference" :default "/Game/Assets/Blueprints/Input/IA_Fire.IA_Fire"))
  (:`Started`
    (bind _pawnref (`self.PawnRef`)
      (:`then`
        (bind _interactref (`/Game/Assets/Blueprints/Player/BP_PawnController.InteractRef` _pawnref)
          (:`then`
            (if (`/Game/Assets/Blueprints/Player/BP_PawnController.IsInteract` _pawnref)
              (message `/Game/Assets/Blueprints/Interface/BPI_Interact.Fire` _interactref)))
          (:`else`)))
      (:`else`)))
  (:`Completed`
    (bind _pawnref_2 (`self.PawnRef`)
      (:`then`
        (bind _interactref_2 (`/Game/Assets/Blueprints/Player/BP_PawnController.InteractRef` _pawnref_2)
          (:`then`
            (if (`/Game/Assets/Blueprints/Player/BP_PawnController.IsInteract` _pawnref_2)
              (message `/Game/Assets/Blueprints/Interface/BPI_Interact.CancelFire` _interactref_2)))
          (:`else`)))
      (:`else`))))

(fn `UserConstructionScript`)