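; AI controller for enemies that runs the BT_Enemie behavior tree on BeginPlay.
; SetEnemieDome stores a dome reference and writes it to the DomeTarget blackboard key.
; Each tick, while the dome is valid, it writes the distance from the controlled pawn to the dome into the Distance key for the behavior tree.
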(event `self.ReceiveBeginPlay`
  (`self.RunBehaviorTree` "/Game/Assets/Blueprints/AI/BT_Enemie.BT_Enemie"))

(event `SetEnemieDome`
  (params (DomeREF :type "/Game/Assets/Blueprints/GamePlay/BP_Dome Object Reference"))
  (bind _output_get (set `self.DomeREF` DomeREF))
  (`BlackboardComponent.SetValueAsObject` (`self.Blackboard`) "DomeTarget" _output_get))

(event `self.ReceiveTick`
  (params (DeltaSeconds :type "Float (single-precision)"))
  (bind _domeref (`self.DomeREF`)
    (:`then`
      (bind _output_get (set `self.Distance` (`KismetMathLibrary.Vector_Distance` (`self.K2_GetActorLocation` (`self.K2_GetPawn`)) (`self.K2_GetActorLocation` _domeref))))
      (`BlackboardComponent.SetValueAsFloat` (`self.Blackboard`) "Distance" _output_get))
    (:`else`)))

(fn `UserConstructionScript`)