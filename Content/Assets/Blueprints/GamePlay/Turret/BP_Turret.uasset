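; BP_Turret is a turret actor that deals continuous hitscan damage straight ahead while firing.
; Fire shows the FireEffect component and starts a fast looping timer, presumably bound to FireHandle, and CancelFire clears the timer and hides the effect.
; FireHandle runs a debug-drawn capsule trace along the actor's forward vector, ignoring REFDome, and applies damage to the hit actor.
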(event `Fire`
  (bind _fireeffect (`self.FireEffect`))
  (bind _returnvalue (`KismetSystemLibrary.K2_SetTimerDelegate` (`|CreateDelegate` :!event `FireHandle`) 0.01 true))
  (set `self.Event_Fire` _returnvalue)
  (`SceneComponent.SetVisibility` _fireeffect true false)
  (`SceneComponent.SetHiddenInGame` _fireeffect false false))

(event `FireHandle`
  (bind _returnvalue (`self.K2_GetActorLocation`))
  (bind (_outhit _returnvalue_2) (`KismetSystemLibrary.CapsuleTraceSingle` _returnvalue (+ _returnvalue (* (`KismetMathLibrary.GetForwardVector` (`self.K2_GetActorRotation`)) 2000)) 10.0 50.0 "TraceTypeQuery1" true (`|MakeArray` (`self.REF_Dome`) :!type "Actor Object Reference") "ForOneFrame"))
  (if _returnvalue_2
    (`GameplayStatics.ApplyDamage` (`.HitActor` (`GameplayStatics.BreakHitResult` _outhit)) 3.0)))

(event `CancelFire`
  (bind _fireeffect (`self.FireEffect`))
  (`KismetSystemLibrary.K2_ClearAndInvalidateTimerHandle` (`self.Event_Fire`))
  (`SceneComponent.SetVisibility` _fireeffect false false)
  (`SceneComponent.SetHiddenInGame` _fireeffect true false))

(fn `UserConstructionScript`)