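; Player-usable dome with Health and Shield that carries a turret along an arc over its top and forwards fire input to it.
; RotateDome shifts a clamped angle, and Tick places the turret via sine/cosine on the sphere's bounds, orienting it with custom atan2 math.
; Items overlapping the box add health and shield by type, then are released from the player and destroyed.
; Text renders show stats and control hints, alongside debug drawing.
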(event OnComponentBeginOverlap(Box)
  (params (OverlappedComponent :type Primitive%20Component%20Object%20Reference) (OtherActor :type Actor%20Object%20Reference) (OtherComp :type Primitive%20Component%20Object%20Reference) (OtherBodyIndex :type Integer) (bFromSweep :type Boolean) (SweepResult :type Hit%20Result%20Structure%20%28by%20ref%29))
  (Class|BPIInteract|SetInteract(Message) OtherActor self)
  (bind _asbp_items (Utilities|Casting|CastToBP_Items OtherActor))
  (Variables|Default|SetHealth (+ (Variables|Default|GetHealth) (Utilities|Select :Index (Variables|/Game/Assets/Blueprints/GamePlay/BP_Items.BP_Items_C|GetType _asbp_items) :NewEnumerator0 5.0 :NewEnumerator1 8.0 :NewEnumerator2 1e+01)))
  (Variables|Default|SetShield (+ (Variables|Default|GetShield) (Utilities|Select :Index (Variables|/Game/Assets/Blueprints/GamePlay/BP_Items.BP_Items_C|GetType _asbp_items) :NewEnumerator0 0.0 :NewEnumerator1 5.0 :NewEnumerator2 8.0)))
  (bind _playerref (Variables|/Game/Assets/Blueprints/GamePlay/BP_Items.BP_Items_C|GetPlayerRef _asbp_items)
    (:then
      (Default|ReleasebyIndex _playerref (Variables|/Game/Assets/Blueprints/GamePlay/BP_Items.BP_Items_C|GetIndexStock _asbp_items)))
    (:else
      _))
  (Actor|DestroyActor _asbp_items))

(event OnComponentEndOverlap(Box)
  (params (OverlappedComponent :type Primitive%20Component%20Object%20Reference) (OtherActor :type Actor%20Object%20Reference) (OtherComp :type Primitive%20Component%20Object%20Reference) (OtherBodyIndex :type Integer))
  (Class|BPIInteract|SetInteract(Message) OtherActor))

(event EventCancelFire
  (bind _turret (Variables|Default|GetTurret)
    (:then
      (Default|CancelFire _turret))
    (:else)))

(event EventRotateDome
  (params (X :type Float%20%28double-precision%29))
  (Variables|Default|SetSpeed (Math|Float|Clamp(Float) (+ X (Variables|Default|GetSpeed)) -9e+01 9e+01)))

(event EventFire
  (bind _turret (Variables|Default|GetTurret)
    (:then
      (Default|Fire _turret))
    (:else)))

(event EventTick
  (params (DeltaSeconds :type Float%20%28single-precision%29))
  (bind _returnvalue (Transformation|GetActorLocation))
  (bind _speed (Variables|Default|GetSpeed))
  (bind _sphere (Variables|Default|GetSphere))
  (bind _debugmode (Variables|Default|GetDebugMode))
  (bind _width (Variables|Default|GetWidth))
  (bind _debugmode_2 (Variables|Default|GetDebugMode))
  (bind _height (Variables|Default|GetHeight))
  (bind _boxextent (Collision|GetComponentBounds _sphere))
  (bind _returnvalue_2 (Math|Float|Clamp(Float) _speed -9e+01 9e+01))
  (bind _returnvalue_3 (Math|Trig|Sin(Degrees) _returnvalue_2))
  (bind _returnvalue_4 (Math|Trig|Cos(Degrees) _returnvalue_2))
  (bind _returnvalue_5 (select _debugmode _width (.y _boxextent)))
  (bind _returnvalue_6 (select _debugmode_2 _height (.z _boxextent)))
  (bind _returnvalue_7 (* _returnvalue_4 _returnvalue_6))
  (bind _returnvalue_8 (* _returnvalue_3 _returnvalue_5))
  (bind _returnvalue_9 (Math|Vector|MakeVector 0.0 _returnvalue_8 _returnvalue_7))
  (Rendering|Components|TextRender|SetText (Variables|Default|GetTextRender) (Utilities|Text|FormatText "Health : {A} 
Shield : {B}" (Variables|Default|GetHealth) (Variables|Default|GetShield)))
  (Rendering|Debug|DrawDebugSphere _returnvalue_9 5e+01 12 "(R=0.779875,G=0.000000,B=1.000000,A=1.000000)" 0.0)
  (bind _turret (Variables|Default|GetTurret)
    (:then
      (Transformation|SetActorLocation _turret (+ _returnvalue_9 (Transformation|GetWorldLocation (Variables|Default|GetSphere))) false false)
      (Transformation|SetActorRotation _turret (CallFunction|GetLookatRotation (Transformation|GetActorLocation _turret) _returnvalue))
      (Rendering|Debug|DrawDebugLine (Transformation|GetActorLocation _turret) _returnvalue "(R=0.000000,G=0.910537,B=1.000000,A=1.000000)" 0.0 5.0))
    (:else)))

(event EventBeginPlay
  (CallFunction|SetTextTuto false)
  (bind _turret (Variables|Default|GetTurret)
    (:then
      (Variables|/Game/Assets/Blueprints/GamePlay/Turret/BP_Turret.BP_Turret_C|SetREF_Dome _turret self))
    (:else)))

(event EventUnUse
  (CallFunction|SetTextTuto false)
  (bind _turret (Variables|Default|GetTurret)
    (:then
      (Default|CancelFire _turret))
    (:else)))

(event EventUse
  (params (Pawn :type BP%20Pawn%20Controller%20Object%20Reference))
  (CallFunction|SetTextTuto true))

(fn ConstructionScript)

(fn SetTextTuto
  (params (isActive :type Boolean))
  (Rendering|Components|TextRender|SetText (Variables|Default|GetTextRender1) (select isActive (Utilities|Text|MakeLiteralText "Left Click : Fire 
A/D : Move 
E : Exit") (Utilities|Text|MakeLiteralText "E : Enter"))))

(fn GetLookatRotation
  (params (Start :type Vector) (Target :type Vector))
  (bind _output_get (LocalVariables|SetDirection (- Start Target)))
  (bind _output_get_2 (LocalVariables|SetAngle (|((atan2(directionY,DirectionX))*Rad2Deg) (.Y (Math|Vector|BreakVector _output_get)) (.Z (Math|Vector|BreakVector _output_get)) (|(360/(PI*2)) (Math|Trig|GetPI)))))
  (Rendering|Debug|DrawDebugLine Start Target "(R=0.197830,G=1.000000,B=0.000000,A=1.000000)" 0.1 5.0)
  (Rendering|Debug|DrawDebugBox (LocalVariables|GetDirection) "10.000000,10.000000,10.000000" "(R=0.000000,G=0.057013,B=1.000000,A=1.000000)" (Math|Rotator|MakeRotator 0.0 (- (Math|Float|Absolute(Float) _output_get_2) 2.7e+02) (select (<= _output_get_2 0.0) 9e+01 -9e+01)) 0.1 1.0)
  (return (Math|Rotator|MakeRotator 0.0 (- (Math|Float|Absolute(Float) _output_get_2) 2.7e+02) (select (<= _output_get_2 0.0) 9e+01 -9e+01))))

(fn GetRotfromX
  (params (Normalize :type Vector))
  (LocalVariables|SetUpVector (select (< (Math|Float|Absolute(Float) (.Z (Math|Vector|BreakVector Normalize))) (- 1.0 1e-05)) "0.000000,0.000000,1.000000" "1.000000,0.000000,0.000000"))
  (LocalVariables|SetNewY (CallFunction|GetNormalize (Math|Vector|MakeVector (|((Y*VZ)-(Z*VY)) (.y (LocalVariables|GetUpVector)) (.z Normalize) (.z (LocalVariables|GetUpVector)) (.y Normalize)) (|((Z*VX)-(X*VZ)) (.z (LocalVariables|GetUpVector)) (.x Normalize) (.x (LocalVariables|GetUpVector)) (.z Normalize)) (|((X*VY)-(Y*VX)) (.x (LocalVariables|GetUpVector)) (.y Normalize) (.y (LocalVariables|GetUpVector)) (.x Normalize))) 0.0001))
  (LocalVariables|SetNewZ (Math|Vector|MakeVector (|((Y*VZ)-(Z*VY)) (.y Normalize) (.z (LocalVariables|GetNewY)) (.z Normalize) (.y (LocalVariables|GetNewY))) (|((Z*VX)-(X*VZ)) (.z Normalize) (.x (LocalVariables|GetNewY)) (.x Normalize) (.z (LocalVariables|GetNewY))) (|((X*VY)-(Y*VX)) (.x Normalize) (.y (LocalVariables|GetNewY)) (.y Normalize) (.x (LocalVariables|GetNewY)))))
  (return (Utilities|Struct|MakeMatrix (Utilities|Struct|MakePlane 0.0 (.x Normalize) (.y Normalize) (.z Normalize)) (Utilities|Struct|MakePlane 0.0 (.x (LocalVariables|GetNewY)) (.y (LocalVariables|GetNewY)) (.z (LocalVariables|GetNewY))) (Utilities|Struct|MakePlane 0.0 (.x (LocalVariables|GetNewZ)) (.y (LocalVariables|GetNewZ)) (.z (LocalVariables|GetNewZ))) (Utilities|Struct|MakePlane 0.0 0.0 0.0 0.0))))

(fn GetRotator
  (params (Matrix :type Matrix%20Structure))
  (LocalVariables|SetXAxis (Class|KismetMathLibrary|MatrixGetScaledAxis Matrix "X"))
  (LocalVariables|SetYAxis (Class|KismetMathLibrary|MatrixGetScaledAxis Matrix "Y"))
  (LocalVariables|SetZAxis (Class|KismetMathLibrary|MatrixGetScaledAxis Matrix "Z"))
  (LocalVariables|SetRadToDeg (/ 1.8e+02 (Math|Trig|GetPI)))
  (bind _output_get (LocalVariables|SetRotator (Math|Rotator|MakeRotator (|((Atan2(XAxisZ,(Sqrt(((Square(XAxisX))+(Square(XAxisY)))))))*{F3C976A8-4371-1A14-B24E-47B2AED8FB0D}) (.z (LocalVariables|GetXAxis)) (.x (LocalVariables|GetXAxis)) (.y (LocalVariables|GetXAxis))) (* (Class|KismetMathLibrary|DegAtan2 (.y (LocalVariables|GetXAxis)) (.x (LocalVariables|GetXAxis))) (LocalVariables|GetRadToDeg)) 0.0)))
  (LocalVariables|SetSYAxis (.Y (Math|Rotator|BreakRotIntoAxes _output_get)))
  (bind _output_get_2 (LocalVariables|SetRotator (Math|Rotator|MakeRotator (* (Class|KismetMathLibrary|DegAtan2 (+ (* (.x (LocalVariables|GetZAxis)) (.x (LocalVariables|GetSYAxis))) (* (.y (LocalVariables|GetZAxis)) (.y (LocalVariables|GetSYAxis))) (* (.z (LocalVariables|GetZAxis)) (.z (LocalVariables|GetSYAxis)))) (+ (* (.x (LocalVariables|GetYAxis)) (.x (LocalVariables|GetSYAxis))) (* (.y (LocalVariables|GetYAxis)) (.y (LocalVariables|GetSYAxis))) (* (.z (LocalVariables|GetYAxis)) (.z (LocalVariables|GetSYAxis))))) (LocalVariables|GetRadToDeg)) (.Pitch (Math|Rotator|BreakRotator _output_get)) (.Yaw (Math|Rotator|BreakRotator _output_get)))))
  (return _output_get_2))

(fn GetNormalize
  (params (Vector :type Vector) (Tolerance :type Float%20%28double-precision%29))
  (bind (_x _y _z) (Math|Vector|BreakVector Vector))
  (LocalVariables|SetSquareSum (+ (* _x _x) (* _y _y) (* _z _z)))
  (if (== (LocalVariables|GetSquareSum) 1.0)
    (return Vector)
    (elif (< (LocalVariables|GetSquareSum) Tolerance)
      (return "0, 0, 0")
      (else
        (LocalVariables|SetScale (Math|Vector|MakeVector (Math|Float|Power (LocalVariables|GetSquareSum) -0.5) (Math|Float|Power (LocalVariables|GetSquareSum) -0.5) (Math|Float|Power (LocalVariables|GetSquareSum) -0.5)))
        (return (Math|Vector|MakeVector (* (.x Vector) (.x (LocalVariables|GetScale))) (* (.y Vector) (.y (LocalVariables|GetScale))) (* (.z Vector) (.z (LocalVariables|GetScale)))))))))