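; BP_Items is a resource block (Iron, Water or Cobalt) that a player pawn picks up on contact.
; BeginPlay sets the cube's material from its Type.
; On hit by BP_PawnController, it looks through PlayerRef's physics handles for an empty one, grabs the cube with it and stores the index.
; Tick pins actor and cube to X=0, keeping movement in the YZ plane.
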(event `self.ReceiveBeginPlay`
  (`self.SetupStats`))

(event `self.Cube.OnComponentHit`
  (params (HitComponent :type "PrimitiveComponent Object Reference") (OtherActor :type "Actor Object Reference") (OtherComp :type "PrimitiveComponent Object Reference") (NormalImpulse :type "Vector Structure") (Hit :type "HitResult Structure (by ref)"))
  (cast `/Game/Assets/Blueprints/Player/BP_PawnController` OtherActor)
  (if (not (`self.IsGrabbed`))
    (bind _playerref (`self.PlayerRef`)
      (:`then`
        (for (_array_element _array_index) (`/Game/Assets/Blueprints/Player/BP_PawnController.ArrayHandlePhysics` _playerref)
          (bind _returnvalue (`PhysicsHandleComponent.GetGrabbedComponent` _array_element))
          (`/Engine/EditorBlueprintResources/StandardMacros.IsValid` _returnvalue
            (:`Is Not Valid`
              (if (== _returnvalue self)
                (break)
                (elif (not (`self.IsGrabbed`))
                  (set `self.IsGrabbed` true)
                  (set `self.IndexStock` _array_index)
                  (`PhysicsHandleComponent.GrabComponentAtLocation` _array_element (`self.Cube`) "None" (`self.K2_GetActorLocation`))
                  (break)
                  (else
                    (break))))))))
      (:`else`))))

(event `self.ReceiveTick`
  (params (DeltaSeconds :type "Float (single-precision)"))
  (bind (_returnvalue_x _returnvalue_y _returnvalue_z) (`KismetMathLibrary.BreakVector` (`self.K2_GetActorLocation`)))
  (bind _cube (`self.Cube`))
  (bind (_returnvalue_x_2 _returnvalue_y_2 _returnvalue_z_2) (`KismetMathLibrary.BreakVector` (`SceneComponent.K2_GetComponentLocation` _cube)))
  (`self.K2_SetActorLocation` (`KismetMathLibrary.MakeVector` 0.0 _returnvalue_y _returnvalue_z))
  (`SceneComponent.K2_SetWorldLocation` _cube (`KismetMathLibrary.MakeVector` 0.0 _returnvalue_y_2 _returnvalue_z_2) false false))

(fn `SetupStats`
  (`PrimitiveComponent.SetMaterial` (`self.Cube`) 0 (select `/Game/Assets/Blueprints/GamePlay/Enum/ETypeItem` (`self.Type`) :`NewEnumerator0` "/Game/Assets/Materials/Bloc/M_Bloc_Iron.M_Bloc_Iron" :`NewEnumerator1` "/Game/Assets/Materials/Bloc/M_Bloc_Water.M_Bloc_Water" :`NewEnumerator2` "/Game/Assets/Materials/Bloc/M_Bloc_Cobalt.M_Bloc_Cobalt" :!type "MaterialInterface Object Reference")))

(fn `UserConstructionScript`)