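; BP_Bloc is a breakable resource block that wears down each time a BP_PawnController actor hits its cube.
; Its type sets hit points and material at construction, optionally re-rolled on BeginPlay through nested weighted random checks favoring Normal.
; At zero hit points it destroys itself once, first spawning a typed BP_Items pickup linked to that pawn for Iron, Water and Cobalt blocks only.
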(event `self.ReceiveBeginPlay`
  (if (`self.RandomBloc`)
    (`self.RandomType`)
    (`self.UpdateStats`)))

(event `self.Cube.OnComponentHit`
  (params (HitComponent :type "PrimitiveComponent Object Reference") (OtherActor :type "Actor Object Reference") (OtherComp :type "PrimitiveComponent Object Reference") (NormalImpulse :type "Vector Structure") (Hit :type "HitResult Structure (by ref)"))
  (bind _asbp_pawn_controller (cast `/Game/Assets/Blueprints/Player/BP_PawnController` OtherActor))
  (`/Engine/EditorBlueprintResources/StandardMacros.DecrementInt` (`self.Hard`)
    (:`  `
      (if (<= (`self.Hard`) 0)
        (`/Engine/EditorBlueprintResources/StandardMacros.DoOnce` false
          (:`Completed`
            (`self.SpawnItem` _asbp_pawn_controller)
            (`self.K2_DestroyActor`)))))))

(fn `RandomType`
  (if (`KismetMathLibrary.RandomBoolWithWeight` 0.5)
    (set `self.TypeBloc` "NewEnumerator0")
    (elif (`KismetMathLibrary.RandomBoolWithWeight` 0.3)
      (set `self.TypeBloc` "NewEnumerator1")
      (elif (`KismetMathLibrary.RandomBoolWithWeight` 0.1)
        (set `self.TypeBloc` "NewEnumerator2")
        (elif (`KismetMathLibrary.RandomBoolWithWeight` 0.06)
          (set `self.TypeBloc` "NewEnumerator3")
          (elif (`KismetMathLibrary.RandomBoolWithWeight` 0.04)
            (set `self.TypeBloc` "NewEnumerator4")
            (else
              (set `self.TypeBloc` "NewEnumerator0"))))))))

(fn `SpawnItem`
  (params (PC :type "/Game/Assets/Blueprints/Player/BP_PawnController Object Reference"))
  (if (and (`|EnumInequality` (`self.TypeBloc`) "NewEnumerator0") (`|EnumInequality` (`self.TypeBloc`) "NewEnumerator1"))
    (`|SpawnActorFromClass` "/Game/Assets/Blueprints/GamePlay/BP_Items.BP_Items_C" (`KismetMathLibrary.MakeTransform` (`self.K2_GetActorLocation`)) "AlwaysSpawn" "MultiplyWithRoot" null PC (select `/Game/Assets/Blueprints/GamePlay/Enum/ETypeBlock` (`self.TypeBloc`) :`NewEnumerator0` "NewEnumerator0" :`NewEnumerator1` "NewEnumerator0" :`NewEnumerator2` "NewEnumerator0" :`NewEnumerator3` "NewEnumerator1" :`NewEnumerator4` "NewEnumerator2" :!type "/Game/Assets/Blueprints/GamePlay/Enum/ETypeItem Enum") null)))

(fn `UpdateStats`
  (bind _typebloc (`self.TypeBloc`))
  (set `self.Hard` (select `/Game/Assets/Blueprints/GamePlay/Enum/ETypeBlock` _typebloc :`NewEnumerator0` 10 :`NewEnumerator1` 50 :`NewEnumerator2` 100 :`NewEnumerator3` 150 :`NewEnumerator4` 180))
  (`PrimitiveComponent.SetMaterial` (`self.Cube`) 0 (select `/Game/Assets/Blueprints/GamePlay/Enum/ETypeBlock` _typebloc :`NewEnumerator0` "/Game/Assets/Materials/Bloc/M_Bloc_Normal.M_Bloc_Normal" :`NewEnumerator1` "/Game/Assets/Materials/Bloc/M_Bloc_Hard.M_Bloc_Hard" :`NewEnumerator2` "/Game/Assets/Materials/Bloc/M_Bloc_Iron.M_Bloc_Iron" :`NewEnumerator3` "/Game/Assets/Materials/Bloc/M_Bloc_Water.M_Bloc_Water" :`NewEnumerator4` "/Game/Assets/Materials/Bloc/M_Bloc_Cobalt.M_Bloc_Cobalt" :!type "MaterialInterface Object Reference")))

(fn `UserConstructionScript`
  (`self.UpdateStats`))