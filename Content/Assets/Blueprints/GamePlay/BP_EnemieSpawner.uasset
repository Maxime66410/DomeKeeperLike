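; Enemy spawner that releases a wave of BP_Enemie actors every two minutes.
; A looping one-second timer decrements a countdown, which on expiry resets, rolls a random wave size and calls SpawnEnemie.
; Each enemy spawns at a randomly picked SpawnA or SpawnB location, ignoring collision, and its AIC_CustomAI controller receives the DomeREF reference.
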(event `self.ReceiveBeginPlay`
  (set `self.Timer` 120.0)
  (set `self.ArraySpawn` (`|MakeArray` (`self.SpawnA`) (`self.SpawnB`)))
  (bind _returnvalue (`KismetSystemLibrary.K2_SetTimerDelegate` (`|CreateDelegate` :!event `CountSpawnEnemie`) 1.0 true))
  (set `self.Event_CountSpawnEnemie` _returnvalue))

(event `CountSpawnEnemie`
  (`/Engine/EditorBlueprintResources/StandardMacros.DecrementFloat` (`self.Timer`)
    (:`  `
      (if (<= (`self.Timer`) 0.0)
        (set `self.Timer` 120.0)
        (set `self.NbrSpawn` (`KismetMathLibrary.RandomIntegerInRange` 3 15))
        (`self.SpawnEnemie`)))))

(event `SpawnEnemie`
  (for _ (range (+ (`self.NbrSpawn`) 1))
    (bind _returnvalue (`|SpawnActorFromClass` "/Game/Assets/Blueprints/AI/BP_Enemie.BP_Enemie_C" (`KismetMathLibrary.MakeTransform` (`SceneComponent.K2_GetComponentLocation` (`KismetArrayLibrary.Array_Random` (`self.ArraySpawn`)))) "AlwaysSpawn" "MultiplyWithRoot" null null))
    (bind _asaic_custom_ai (cast `/Game/Assets/Blueprints/AI/AIC_CustomAI` (`AIBlueprintHelperLibrary.GetAIController` _returnvalue)))
    (`/Game/Assets/Blueprints/AI/AIC_CustomAI.SetEnemieDome` _asaic_custom_ai (`self.DomeREF`))))

(fn `UserConstructionScript`)